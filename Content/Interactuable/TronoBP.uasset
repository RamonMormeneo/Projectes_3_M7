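; TronoBP is an interactable throne actor (per its name and folder) that shows a hover prompt and a text box.
; Its Box trigger creates a Hover widget when the ThirdPersonCharacter enters and removes it on exit.
; The Open event, not called within this graph, removes that hover and adds a TextBoxLibreta33 widget to the viewport.
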(event `self.ReceiveBeginPlay`)

(event `Open`
  (`Widget.RemoveFromParent` (`self.NewVar_0`))
  (bind _returnvalue (`|CreateWidget` "/Game/TextBox/TextBoxLibreta33.TextBoxLibreta33_C"))
  (`UserWidget.AddToViewport` _returnvalue 0))

(event `self.Box.OnComponentEndOverlap`
  (params (OverlappedComponent :type "PrimitiveComponent Object Reference") (OtherActor :type "Actor Object Reference") (OtherComp :type "PrimitiveComponent Object Reference") (OtherBodyIndex :type Integer))
  (cast `/Game/ThirdPersonBP/Blueprints/ThirdPersonCharacter` OtherActor)
  (`/Engine/EditorBlueprintResources/StandardMacros.IsValid` (`self.NewVar_0`)
    (:`Is Valid`
      (`Widget.RemoveFromParent` (`self.NewVar_0`)))))

(event `self.Box.OnComponentBeginOverlap`
  (params (OverlappedComponent :type "PrimitiveComponent Object Reference") (OtherActor :type "Actor Object Reference") (OtherComp :type "PrimitiveComponent Object Reference") (OtherBodyIndex :type Integer) (bFromSweep :type Boolean) (SweepResult :type "HitResult Structure (by ref)"))
  (cast `/Game/ThirdPersonBP/Blueprints/ThirdPersonCharacter` OtherActor)
  (bind _returnvalue (`|CreateWidget` "/Game/TextBox/Hover.Hover_C"))
  (set `self.NewVar_0` _returnvalue)
  (`UserWidget.AddToViewport` _returnvalue 0))

(fn `UserConstructionScript`)